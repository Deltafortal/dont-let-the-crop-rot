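; Farmable hoed soil actor where seeds are planted, watered and harvested into the character's inventory.
; Seeds from the item data table set named timers that swap placeholder meshes through planted, growing and mature stages.
; Watering restarts the drought timer; expiry halts growth and leaves a dried plant that yields nothing.
; Interacting harvests ready plants; using a seed on a ready plant harvests and replants.
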(event `/Game/MyContent/Blueprints/Interfaces/BPI_Interact.InteractWith`
  (params (Character :type "/Game/ThirdPerson/Blueprints/BP_ThirdPersonCharacter Object Reference"))
  (set `self.Character` Character)
  (`self.Harvest`))

(event `/Game/MyContent/Blueprints/Interfaces/BPI_Interact.UseOnActor`
  (params (ItemUsed :type Name) (Character :type "/Game/ThirdPerson/Blueprints/BP_ThirdPersonCharacter Object Reference"))
  (set `self.Character` Character)
  (bind _output_get (set `self.ItemUsed` ItemUsed))
  (bind _returnvalue (`|GetDataTableRow` "/Game/MyContent/Blueprints/Data/DataTables/ItemDataTable.ItemDataTable" _output_get)
    (:`then`
      (bind (_name _description _icon _maxstacksize _actiontype _issellable _price _weapondata _tooldata _decorationdata _consumabledata _defensedata _seeddata _placeactor _itemfamily) (break `/Game/MyContent/Blueprints/Data/DataStructs/F_ItemStruct` _returnvalue))
      (switch `/Game/MyContent/Blueprints/Data/Enums/En_ItemFamily` _itemfamily
        (:`NewEnumerator0`
          ; Watering
          (if (== (`self.ItemUsed`) (`self.WateringCanRowName`))
            (if (`self.IsPlanted`)
              (`KismetSystemLibrary.K2_ClearTimer` null "DryPlant")
              (`KismetSystemLibrary.K2_SetTimer` null "DryPlant" (`self.DryTime`)))))
        (:`NewEnumerator1`
          (set `self.Seed Data` _seeddata)
          (if (`self.IsPlanted`)
            (`self.Harvest`)
            ; Place Another Seed
            (`self.UseOnActor` self (`self.ItemUsed`) (`self.Character`))
            (else
              (set `self.IsPlanted` true)
              (`/Game/MyContent/Blueprints/Components/BP_InventoryComponent.RemoveItem` (`/Game/ThirdPerson/Blueprints/BP_ThirdPersonCharacter.BP_InventoryComponent` (`self.Character`)) (`self.ItemUsed`) 1)
              (`self.PlantedStage`))))))))

(fn `DryPlant`
  (set `self.IsDrought` true)
  (`StaticMeshComponent.SetStaticMesh` (`self.Plant`) "/Engine/EngineMeshes/SM_MatPreviewMesh_01.SM_MatPreviewMesh_01")
  (`KismetSystemLibrary.K2_ClearTimer` null "GrowingStage")
  (`KismetSystemLibrary.K2_ClearTimer` null "MaturingStage")
  (set `self.IsReadyHarvest` true))

(fn `GrowingStage`
  (`KismetSystemLibrary.PrintString` "Plant has Grown" true true (struct :`R` 1.0 :`G` 0.35524 :`B` 0.855352 :`A` 1.0))
  (`StaticMeshComponent.SetStaticMesh` (`self.Plant`) "/Engine/EngineMeshes/Sphere.Sphere")
  (`KismetSystemLibrary.K2_SetTimer` null "MaturingStage" (`self.GrowingTime`)))

(fn `Harvest`
  (bind (_growthdays _droughtdays _rotresistance _goldenharvestchance _droppingseedchance _seedtier _itemdrop _quantitytodrop) (break `/Game/MyContent/Blueprints/Data/DataStructs/F_SeedStruct` (`self.Seed Data`)))
  (if (`self.IsReadyHarvest`)
    (`StaticMeshComponent.SetStaticMesh` (`self.Plant`) null)
    (`KismetSystemLibrary.K2_ClearTimer` null "DryPlant")
    (set `self.IsReadyHarvest` false)
    (set `self.IsPlanted` false)
    (if (`self.IsDrought`)
      ;[0.15 0.02308 0.04446 0.5] Waste Plant
      (set `self.IsRot` false)
      (set `self.IsDrought` false)
      (else
        ;[0.06378 0.15 0.06273 0.5] Get Grow Plant
        (`/Game/MyContent/Blueprints/Components/BP_InventoryComponent.AddItem` (`/Game/ThirdPerson/Blueprints/BP_ThirdPersonCharacter.BP_InventoryComponent` (`self.Character`)) _itemdrop _quantitytodrop)))))

(fn `MaturingStage`
  (`KismetSystemLibrary.PrintString` "Plant Ready to Harvest" true true (struct :`R` 1.0 :`G` 0.35524 :`B` 0.855352 :`A` 1.0))
  (`StaticMeshComponent.SetStaticMesh` (`self.Plant`) "/Engine/BasicShapes/Cube.Cube")
  (set `self.IsReadyHarvest` true))

(fn `PlantedStage`
  (bind (_growthdays _droughtdays) (break `/Game/MyContent/Blueprints/Data/DataStructs/F_SeedStruct` (`self.Seed Data`)))
  (`KismetSystemLibrary.PrintString` "Seed Planted" true true (struct :`R` 1.0 :`G` 0.35524 :`B` 0.855352 :`A` 1.0))
  (`StaticMeshComponent.SetStaticMesh` (`self.Plant`) "/Engine/BasicShapes/Cone.Cone")
  ; Set Seed Info
  (set `self.GrowingTime` (/ (`KismetMathLibrary.Conv_IntToDouble` _growthdays) 2.0))
  (set `self.DryTime` (`KismetMathLibrary.Conv_IntToDouble` _droughtdays))
  (`KismetSystemLibrary.K2_SetTimer` null "DryPlant" (`self.DryTime`))
  (`KismetSystemLibrary.K2_SetTimer` null "GrowingStage" (`self.GrowingTime`)))

(fn `UserConstructionScript`)