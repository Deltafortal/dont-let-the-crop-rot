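; BP_OcclusionField is a volume that fades out a nearby roof while an actor overlaps it.
; Its construction script sizes the box from extent variables.
; On any overlap, a sphere trace at the root stores the hit component as HitRoof and lowers Opacity on a dynamic instance of its first material.
; End overlap restores full opacity on HitRoof, again through a create-instance call.
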(event `self.ReceiveActorBeginOverlap`
  (params (OtherActor :type "Actor Object Reference"))
  (bind _returnvalue (`SceneComponent.K2_GetComponentLocation` (`self.DefaultSceneRoot`)))
  (bind _outhit (`KismetSystemLibrary.SphereTraceSingle` _returnvalue _returnvalue 120.0 "TraceTypeQuery1"))
  (bind _output_get (set `self.HitRoof` (`.HitComponent` (`GameplayStatics.BreakHitResult` _outhit))))
  (bind _returnvalue_2 (`PrimitiveComponent.CreateDynamicMaterialInstance` _output_get 0 (`PrimitiveComponent.GetMaterial` (`self.HitRoof`) 0) "None"))
  (`MaterialInstanceDynamic.SetScalarParameterValue` _returnvalue_2 "Opacity" 0.1))

(event `self.ReceiveActorEndOverlap`
  (params (OtherActor :type "Actor Object Reference"))
  (bind _returnvalue (`PrimitiveComponent.CreateDynamicMaterialInstance` (`self.HitRoof`) 0 (`PrimitiveComponent.GetMaterial` (`self.HitRoof`) 0) "None"))
  (`MaterialInstanceDynamic.SetScalarParameterValue` _returnvalue "Opacity" 1.0))

(fn `UserConstructionScript`
  ; Extend Volume
  (`BoxComponent.SetBoxExtent` (`self.Box`) (`KismetMathLibrary.MakeVector` (`self.In Box Extent X`) (`self.In Box Extent Y`) (`self.In Box Extent Z`)) true))