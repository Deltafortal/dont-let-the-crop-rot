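; Actor component that stores a player's hotbar as slot structs of item name and quantity, with "None" marking empty slots.
; Adding fills the first empty slot without stacking; removing decrements or clears a matching slot via a custom ElseIf macro.
; Changes reach the owner through messages that update the hotbar or clear the equipped item, while EquipItem returns a data table row handle.
; The Inventory array is only resized, and NEWAddToInventory is an empty stub.
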(event `self.ReceiveBeginPlay`
  ; Initialize Inventory
  (`KismetArrayLibrary.Array_Resize` (`self.Hotbar`) (`self.HotbarSize`))
  (`KismetArrayLibrary.Array_Resize` (`self.Inventory`) (`self.InventorySyze`)))

(fn `AddToInventory`
  (params (ItemToAdd :type Name) (QuantityToAdd :type Integer))
  (for (_array_element _array_index) (`self.Hotbar`)
    (if (== (`.ItemName_15_4D004A314BDAFE90F6C517B210BA9935` (break `/Game/MyContent/Blueprints/Data/DataStructs/F_SlotStruct` _array_element)) "None")
      ;[0.06379 0.15 0.06273 0.5] Add Item To Inventory Slot and Stop the Cycle
      (`KismetArrayLibrary.Array_Set` (`self.Hotbar`) _array_index (make `/Game/MyContent/Blueprints/Data/DataStructs/F_SlotStruct` (`local.ItemToAdd`) (`local.QuantityToAdd`)))
      (`self.CallUpdateHotbar`)
      (break)
      (else
        ;[0.15 0.04925 0.04553 0.5] InventoryFull
        (if (== _array_index (- (`self.HotbarSize`) 1))
          (`KismetSystemLibrary.PrintString` "InventoryFull" true true (struct :`R` 1.0 :`G` 0.030392 :`B` 0.04376 :`A` 1.0)))))))

(fn `CallUpdateHotbar`
  (message `/Game/MyContent/Blueprints/Interfaces/BPI_Hotbar.UpdateHotbar` (`self.GetOwner`) (`self.Hotbar`)))

(fn `DEBUG_PrintInventory`
  (for (_array_element _array_index) (`self.Hotbar`)
    (bind (_itemname _quantity) (break `/Game/MyContent/Blueprints/Data/DataStructs/F_SlotStruct` _array_element))
    (`KismetSystemLibrary.PrintString` (`KismetStringLibrary.Concat_StrStr` "Index: " (`KismetStringLibrary.Conv_IntToString` _array_index) " ItemId: " (`KismetStringLibrary.Conv_NameToString` _itemname) " Quantity: " (`KismetStringLibrary.Conv_IntToString` _quantity)) true true (struct :`R` 0.148288 :`B` 1.0 :`A` 1.0) 5.0)))

(fn `EquipItem`
  (params (SelectedIndex :type Integer))
  (returns (EquippedItem :type "DataTableRowHandle Structure"))
  (return (make `DataTableRowHandle` "/Game/MyContent/Blueprints/Data/DataTables/ItemDataTable.ItemDataTable" (`.ItemName_15_4D004A314BDAFE90F6C517B210BA9935` (break `/Game/MyContent/Blueprints/Data/DataStructs/F_SlotStruct` (`|GetArrayItem` (`self.Hotbar`) SelectedIndex))))))

(fn `NEWAddToInventory`
  (params (ItemToAdd :type Name) (QuantityToAdd :type Integer)))

(fn `RemoveFromInventory`
  (params (ItemToRemove :type Name) (QuantityToRemove :type Integer))
  (locals (IntentoryQuantity :type Integer) (InventoryItemName :type Name) (InventorySlotIndex :type Integer))
  (for (_array_element _array_index) (`self.Hotbar`)
    (set `local.InventorySlotIndex` _array_index)
    (bind (_itemname _quantity) (break `/Game/MyContent/Blueprints/Data/DataStructs/F_SlotStruct` _array_element))
    (set `local.IntentoryQuantity` _quantity)
    (set `local.InventoryItemName` _itemname)
    (if (== _itemname (`local.ItemToRemove`))
      (`self.ElseIf` (> (`local.IntentoryQuantity`) (`local.QuantityToRemove`)) (== (`local.IntentoryQuantity`) (`local.QuantityToRemove`))
        (:`If`
          ;[0.06379 0.15 0.06273 0.5] Reduce Quantity
          (`KismetArrayLibrary.Array_Set` (`self.Hotbar`) (`local.InventorySlotIndex`) (make `/Game/MyContent/Blueprints/Data/DataStructs/F_SlotStruct` (`local.InventoryItemName`) (- (`local.IntentoryQuantity`) (`local.QuantityToRemove`))))
          (`self.CallUpdateHotbar`)
          (break))
        (:`ElseIf`
          ;[0.06379 0.15 0.06273 0.5] Delete Item
          (`KismetArrayLibrary.Array_Set` (`self.Hotbar`) (`local.InventorySlotIndex`) (make `/Game/MyContent/Blueprints/Data/DataStructs/F_SlotStruct` "None"))
          (`self.CallUpdateHotbar`)
          (message `/Game/MyContent/Blueprints/Interfaces/BPI_Inventory.ClearEquippedItem` (`self.GetOwner`) (`local.ItemToRemove`))
          (break))
        (:`Else`
          ;[0.15 0.02308 0.04446 0.5] Not Enough Quantity
          (`KismetSystemLibrary.PrintString` "Not Enough Quantity" true true (struct :`R` 0.992004 :`G` 1.0 :`B` 0.136453 :`A` 1.0)))))))