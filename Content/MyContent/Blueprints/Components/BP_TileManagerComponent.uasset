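; BP_TileManagerComponent is a tile manager component that snaps a position to a square grid.
; GetSnappedPosition rounds X and Y to the nearest multiple of GridSize and raises Z by a tiny fixed offset.
; Its BeginPlay and Tick events are disabled placeholders, so that function is the only logic in the graphs.
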(fn `GetSnappedPosition`
  (params (InputX :type "Float (double-precision)") (InputY :type "Float (double-precision)") (InputZ :type "Float (double-precision)"))
  (returns (OutputX :type "Float (double-precision)") (OutputY :type "Float (double-precision)") (OutputZ :type "Float (double-precision)"))
  (locals (SnappedX :type "Float (double-precision)") (SnappedY :type "Float (double-precision)") (LastIndex :type Integer) (SnappedZ :type "Float (double-precision)"))
  (set `local.SnappedZ` (+ InputZ 0.1))
  (set `local.SnappedY` (* (`KismetMathLibrary.Round` (/ InputY (`self.GridSize`))) (`self.GridSize`)))
  (set `local.SnappedX` (* (`self.GridSize`) (`KismetMathLibrary.Round` (/ InputX (`self.GridSize`)))))
  (return (`local.SnappedX`) (`local.SnappedY`) (`local.SnappedZ`)))